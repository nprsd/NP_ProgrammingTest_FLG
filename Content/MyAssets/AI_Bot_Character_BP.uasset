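; AI bot character Blueprint that drains the player's RedResource while the player is within its Sphere component.
; Sphere begin and end overlap events, filtered to ProgrammingTestCharacter, toggle an IsColliding flag.
; Tick checks that flag and a positive resource, then uses a one-second Delay to throttle subtraction of RedResourceDeduction.
; A pending deduction still applies if the player leaves during the delay, as conditions are not rechecked.
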(event `self.ReceiveTick`
  (params (DeltaSeconds :type "Float (single-precision)"))
  (bind _asprogramming_test_character (cast `ProgrammingTestCharacter` (`GameplayStatics.GetPlayerCharacter` 0)))
  (bind _redresource (`ProgrammingTestCharacter.RedResource` _asprogramming_test_character))
  (if (and (`self.isColliding`) (> _redresource 0))
    (`KismetSystemLibrary.Delay` 1.0)
    (set `ProgrammingTestCharacter.RedResource` (- _redresource (`self.RedResourceDeduction`)) _asprogramming_test_character)))

(event `self.Sphere.OnComponentBeginOverlap`
  (params (OverlappedComponent :type "PrimitiveComponent Object Reference") (OtherActor :type "Actor Object Reference") (OtherComp :type "PrimitiveComponent Object Reference") (OtherBodyIndex :type Integer) (bFromSweep :type Boolean) (SweepResult :type "HitResult Structure (by ref)"))
  (cast `ProgrammingTestCharacter` OtherActor)
  (set `self.isColliding` true))

(event `self.Sphere.OnComponentEndOverlap`
  (params (OverlappedComponent :type "PrimitiveComponent Object Reference") (OtherActor :type "Actor Object Reference") (OtherComp :type "PrimitiveComponent Object Reference") (OtherBodyIndex :type Integer))
  (cast `ProgrammingTestCharacter` OtherActor)
  (set `self.isColliding` false))

(fn `UserConstructionScript`)